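; BP_Bullet is a projectile that damages the player on contact.
; Each Tick moves it by normalized Direction times Speed as a local offset, without sweep or delta-time scaling, so its speed depends on frame rate.
; A Delay on Tick destroys it once BulletLifetime elapses.
; Overlapping the player pawn cached at BeginPlay calls DamagePlayer, then destroys the bullet after a short delay; other actors are ignored.
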(event OnComponentBeginOverlap(SM_Bullet)
  (params (OverlappedComponent :type Primitive%20Component%20Object%20Reference) (OtherActor :type Actor%20Object%20Reference) (OtherComp :type Primitive%20Component%20Object%20Reference) (OtherBodyIndex :type Integer) (bFromSweep :type Boolean) (SweepResult :type Hit%20Result%20Structure%20%28by%20ref%29))
  (bind _playerreference (Variables|Default|GetPlayerReference))
  ;[0.849 0.36 0.2849 0.5] Damage Player & Destroy Bullet
  (if (== OtherActor _playerreference)
    (Default|DamagePlayer _playerreference (Variables|Default|GetDamage))
    (Utilities|FlowControl|Delay 0.2)
    (Actor|DestroyActor)))

(event EventBeginPlay
  ;[0.4146 0.6753 0.3248 0.5] Get Player Reference
  (bind _asbp_third_person_character (Utilities|Casting|CastToBP_ThirdPersonCharacter (Game|Player|GetPlayerPawn 0)))
  (Variables|Default|SetPlayerReference _asbp_third_person_character))

(event EventTick
  (params (DeltaSeconds :type Float%20%28single-precision%29))
  ;[0.2781 0.7969 0.5337 0.5] Bullet Movement
  (Transformation|AddActorLocalOffset (* (Math|Vector|Normalize (Variables|Default|GetDirection)) (Variables|Default|GetSpeed)) false false)
  ;[0.2781 0.7969 0.5337 0.5] Destroy Bullet after Lifetime has Elapsed
  (Utilities|FlowControl|Delay (Variables|Default|GetBulletLifetime))
  (Actor|DestroyActor))

(fn ConstructionScript)