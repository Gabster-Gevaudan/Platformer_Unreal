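; BP_Enemy_Path is a platformer enemy that walks a spider mesh along a spline path, looping endlessly from BeginPlay.
; A timeline, with play rate set from the Speed variable, maps its alpha to distance along the EnemyPath spline.
; Each update moves the mesh to that spline transform, with yaw turned 180 degrees.
; When the timeline finishes, Walk restarts it from the beginning.
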(event Custom|Walk
  ;[0.15 0.15 0.15 0.5] Walk Pathing
  (Components|Timeline|SetPlayRate (Variables|Default|GetWalkTimeline) (Variables|Default|GetSpeed))
  (bind _walktrack (Timeline|WalkTimeline PlayFromStart)
    (:Update
      (Transformation|SetWorldLocationAndRotation (Variables|Default|GetSM_Spider_01) (.location (Spline|GetTransformatDistanceAlongSpline (Variables|Default|GetEnemy_Path) (Math|Float|Lerp 0.0 (Spline|GetSplineLength (Variables|Default|GetEnemy_Path)) _walktrack) "World" false)) (Math|Rotator|MakeRotator (.roll (.rotation (Spline|GetTransformatDistanceAlongSpline (Variables|Default|GetEnemy_Path) (Math|Float|Lerp 0.0 (Spline|GetSplineLength (Variables|Default|GetEnemy_Path)) _walktrack) "World" false))) (.pitch (.rotation (Spline|GetTransformatDistanceAlongSpline (Variables|Default|GetEnemy_Path) (Math|Float|Lerp 0.0 (Spline|GetSplineLength (Variables|Default|GetEnemy_Path)) _walktrack) "World" false))) (- (.yaw (.rotation (Spline|GetTransformatDistanceAlongSpline (Variables|Default|GetEnemy_Path) (Math|Float|Lerp 0.0 (Spline|GetSplineLength (Variables|Default|GetEnemy_Path)) _walktrack) "World" false))) 1.8e+02)) false false))
    (:Finished
      (CallFunction|Walk))))

(event EventBeginPlay
  ;[0.15 0.15 0.15 0.5] Setup
  (CallFunction|Walk))

(fn ConstructionScript)