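; Chaser enemy that pursues the player while they are inside its detection zone and scatters a random number of coins on death.
; Tick yaws it toward the player and feeds straight-line movement input, without pathfinding.
; Player overlaps with the hit zone launch the player and cost the enemy one health, destroying it at zero.
; Capsule hits damage the player and knock them back along the enemy's velocity.
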(event OnComponentBeginOverlap(DetectionZone)
  (params (OverlappedComponent :type Primitive%20Component%20Object%20Reference) (OtherActor :type Actor%20Object%20Reference) (OtherComp :type Primitive%20Component%20Object%20Reference) (OtherBodyIndex :type Integer) (bFromSweep :type Boolean) (SweepResult :type Hit%20Result%20Structure%20%28by%20ref%29))
  ;[1 0.6196 0.9732 0.5] Check if Detecting Player
  (if (== OtherActor (Variables|Default|GetPlayer%20Reference))
    (Variables|Default|SetCanDetectPlayer true)))

(event OnComponentEndOverlap(DetectionZone)
  (params (OverlappedComponent :type Primitive%20Component%20Object%20Reference) (OtherActor :type Actor%20Object%20Reference) (OtherComp :type Primitive%20Component%20Object%20Reference) (OtherBodyIndex :type Integer))
  ;[1 0.6196 0.9732 0.5] Check if Detecting Player
  (if (== OtherActor (Variables|Default|GetPlayer%20Reference))
    (Variables|Default|SetCanDetectPlayer false)))

(event OnComponentBeginOverlap(HitZone)
  (params (OverlappedComponent :type Primitive%20Component%20Object%20Reference) (OtherActor :type Actor%20Object%20Reference) (OtherComp :type Primitive%20Component%20Object%20Reference) (OtherBodyIndex :type Integer) (bFromSweep :type Boolean) (SweepResult :type Hit%20Result%20Structure%20%28by%20ref%29))
  ;[0.75 0.5 1 0.5] If the Player is in the Hit Zone...
  (if (== OtherActor (Variables|Default|GetPlayer%20Reference))
    (Utilities|FlowControl|Sequence
      (:then_0
        ;[0.75 0.5 1 0.5] Launch Player
        (Character|LaunchCharacter (Variables|Default|GetPlayer%20Reference) (Variables|Default|GetLaunchDirection) false false))
      (:then_1
        ;[0.75 0.5 1 0.5] Calculate Enemy Health
        (Variables|Default|SetHealth (- (Variables|Default|GetHealth) 1))
        ;[0.75 0.5 1 0.5] Destroy Enemy
        (if (<= (Variables|Default|GetHealth) 0)
          (CallFunction|LootandDestroy))))))

(event OnComponentHit(CapsuleComponent)
  (params (HitComponent :type Primitive%20Component%20Object%20Reference) (OtherActor :type Actor%20Object%20Reference) (OtherComp :type Primitive%20Component%20Object%20Reference) (NormalImpulse :type Vector :default "0, 0, 0") (Hit :type Hit%20Result%20Structure%20%28by%20ref%29))
  ;[1 0.5 0.25 0.5] Knockback Attack
  (if (== OtherActor (Variables|Default|GetPlayer%20Reference))
    (Character|LaunchCharacter (Variables|Default|GetPlayer%20Reference) (* (Transformation|GetVelocity) (Variables|Default|GetKnockbackStrength)) false false)
    ;[1 0.5 0.25 0.5] Damage Player
    (Default|DamagePlayer (Variables|Default|GetPlayer%20Reference) (Variables|Default|GetPlayerDamage))))

(event Custom|LootAndDestroy
  (bind _returnvalue (Transformation|GetActorTransform))
  ;[1 0.75 0.15 0.5] Loot & Destroy
  (for _index (range 0 (Math|Random|RandomIntegerinRange 0 (Variables|Default|GetCoinsDropped)))
    (Game|SpawnActorfromClass "/Game/Platformer/Blueprints/BP_Coin.BP_Coin_C" (Math|Transform|MakeTransform (Math|Vector|MakeVector (+ (Math|Random|RandomFloatinRange -2e+02 2e+02) (.x (.location _returnvalue))) (+ (Math|Random|RandomFloatinRange -2e+02 2e+02) (.y (.location _returnvalue))) (.z (.location _returnvalue))) (.rotation _returnvalue) (.scale _returnvalue)) "Undefined" "MultiplyWithRoot" 0 0))
  (Actor|DestroyActor))

(event EventBeginPlay
  ;[0.5865 0.8333 0.3429 0.5] Get Player Reference
  (bind _asbp_third_person_character (Utilities|Casting|CastToBP_ThirdPersonCharacter (Game|Player|GetPlayerPawn 0)))
  (Variables|Default|SetPlayer%20Reference _asbp_third_person_character))

(event EventTick
  (params (DeltaSeconds :type Float%20%28single-precision%29))
  (bind _returnvalue (Transformation|GetActorLocation))
  (bind _player_reference (Variables|Default|GetPlayer%20Reference))
  (bind _returnvalue_2 (Transformation|GetActorLocation _player_reference))
  ;[0.25 0.75 1 0.5] If Player is Detected...
  (if (Variables|Default|GetCanDetectPlayer)
    (Utilities|FlowControl|Sequence
      (:then_0
        ;[0.25 0.75 1 0.5] Look at Player
        (Transformation|SetActorRotation (Math|Rotator|FindLookatRotation (Math|Vector|MakeVector (.x _returnvalue) (.y _returnvalue) 0.0) (Math|Vector|MakeVector (.x _returnvalue_2) (.y _returnvalue_2) 0.0))))
      (:then_1
        ;[0.25 0.75 1 0.5] Chase Player
        (Pawn|Input|AddMovementInput (Math|Vector|Normalize (- (Transformation|GetActorLocation (Variables|Default|GetPlayer%20Reference)) (Transformation|GetActorLocation))) 1.0 false)))))

(fn ConstructionScript)