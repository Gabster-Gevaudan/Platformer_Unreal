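; Platformer platform that vanishes after the player stands on it for a set lifetime, then reappears.
; A trigger zone flags the player pawn's presence, and Tick accumulates time on the platform, resetting it when the player is off.
; At the lifetime limit the actor hides and disables collision, then after a delay restores its BeginPlay transform, visibility and collision.
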(event OnComponentBeginOverlap(PlatformTriggerZone)
  (params (OverlappedComponent :type Primitive%20Component%20Object%20Reference) (OtherActor :type Actor%20Object%20Reference) (OtherComp :type Primitive%20Component%20Object%20Reference) (OtherBodyIndex :type Integer) (bFromSweep :type Boolean) (SweepResult :type Hit%20Result%20Structure%20%28by%20ref%29))
  ;[1 0.7135 0.7858 0.5] Collider Check
  (if (== OtherActor (Game|Player|GetPlayerPawn 0))
    (Variables|Default|SetIsPlayerOnPlatform true)))

(event OnComponentEndOverlap(PlatformTriggerZone)
  (params (OverlappedComponent :type Primitive%20Component%20Object%20Reference) (OtherActor :type Actor%20Object%20Reference) (OtherComp :type Primitive%20Component%20Object%20Reference) (OtherBodyIndex :type Integer))
  ;[1 0.7135 0.7858 0.5] Collider Check
  (if (== OtherActor (Game|Player|GetPlayerPawn 0))
    (Variables|Default|SetIsPlayerOnPlatform false)))

(event Custom|Return%20To%20Start
  ;[0.8294 0.8438 0.2505 0.5] Return to Start
  (Transformation|SetWorldTransform (Variables|Default|GetDefaultSceneRoot) (Variables|Default|GetStartTransform) false true)
  (Variables|Default|SetTimeOnPlatform 0.0)
  (Rendering|SetActorHiddenInGame false)
  (Collision|SetActorEnableCollision true))

(event EventBeginPlay
  ;[0.2721 0.5304 0.2721 0.5] Set Start Position, Rotation, Scale
  (Variables|Default|SetStartTransform (Transformation|GetActorTransform)))

(event EventTick
  (params (DeltaSeconds :type Float%20%28single-precision%29))
  ;[0.1839 0.3733 0.6615 0.5] Set Timer For Platform
  (if (Variables|Default|GetIsPlayerOnPlatform)
    (Variables|Default|SetTimeOnPlatform (+ (Variables|Default|GetTimeOnPlatform) DeltaSeconds))
    ;[0.1839 0.3733 0.6615 0.5] Check if Timer has reached the Platform's life time
    (if (>= (Variables|Default|GetTimeOnPlatform) (Variables|Default|GetPlatformLifetime))
      ;[0.1839 0.3733 0.6615 0.5] Hide & Disable Platform
      (Rendering|SetActorHiddenInGame true)
      (Collision|SetActorEnableCollision false)
      (Utilities|FlowControl|Delay (Variables|Default|GetTimeInvisible))
      (CallFunction|ReturntoStart))
    (else
      (Variables|Default|SetTimeOnPlatform 0.0))))

(fn ConstructionScript)