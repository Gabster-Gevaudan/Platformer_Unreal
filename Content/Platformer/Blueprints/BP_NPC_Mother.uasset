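; BP_NPC_Mother is a talkable NPC for the platformer that shows dialogue lines through the player character.
; A trigger zone shows or hides an interaction prompt widget as the player enters or leaves.
; ResetDialogue restarts the sequence, and UpdateDialogue recursively writes each line into the player's CurrentDialogueText on a fixed delay, clearing it after the last line.
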(event OnComponentBeginOverlap(NPCTriggerZone)
  (params (OverlappedComponent :type Primitive%20Component%20Object%20Reference) (OtherActor :type Actor%20Object%20Reference) (OtherComp :type Primitive%20Component%20Object%20Reference) (OtherBodyIndex :type Integer) (bFromSweep :type Boolean) (SweepResult :type Hit%20Result%20Structure%20%28by%20ref%29))
  ;[0.7448 0.4787 0.568 0.5] Enable / Disable Widget
  (if (== OtherActor (Variables|Default|GetPlayer%20Reference))
    (Rendering|SetVisibility (Variables|Default|GetInteraction%20Prompt%20Widget) true false)))

(event OnComponentEndOverlap(NPCTriggerZone)
  (params (OverlappedComponent :type Primitive%20Component%20Object%20Reference) (OtherActor :type Actor%20Object%20Reference) (OtherComp :type Primitive%20Component%20Object%20Reference) (OtherBodyIndex :type Integer))
  ;[0.7448 0.4787 0.568 0.5] Enable / Disable Widget
  (if (== OtherActor (Variables|Default|GetPlayer%20Reference))
    (Rendering|SetVisibility (Variables|Default|GetInteraction%20Prompt%20Widget) false false)))

(event Custom|UpdateDialogue
  ;[0.2595 0.5333 0.6337 0.5] Update Dialogue
  (Variables|/Game/Platformer/Blueprints/BP_ThirdPersonCharacter.BP_ThirdPersonCharacter_C|SetCurrentDialogueText (Variables|Default|GetPlayer%20Reference) (Utilities|Array|Get(acopy) (Variables|Default|GetDialogueLines) (Variables|Default|GetCurrentDialogueLine)))
  (Variables|Default|SetCurrentDialogueLine (+ (Variables|Default|GetCurrentDialogueLine) 1))
  (Utilities|FlowControl|Delay 2.0)
  (if (!= (Variables|Default|GetCurrentDialogueLine) (Utilities|Array|Length (Variables|Default|GetDialogueLines)))
    (CallFunction|UpdateDialogue)
    (else
      (Variables|/Game/Platformer/Blueprints/BP_ThirdPersonCharacter.BP_ThirdPersonCharacter_C|SetCurrentDialogueText (Variables|Default|GetPlayer%20Reference) ""))))

(event Custom|ResetDialogue
  ;[0.2321 0.365 0.6337 0.5] Reset Dialogue
  (Variables|Default|SetCurrentDialogueLine 0)
  (CallFunction|UpdateDialogue))

(event EventBeginPlay
  ;[0.3342 0.6615 0.393 0.5] Create a Player Reference
  (bind _asbp_third_person_character (Utilities|Casting|CastToBP_ThirdPersonCharacter (Game|Player|GetPlayerPawn 0)))
  (Variables|Default|SetPlayer%20Reference _asbp_third_person_character))

(fn ConstructionScript)