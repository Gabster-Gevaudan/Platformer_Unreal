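; Platform hazard that knocks back and damages the player on contact.
; On BeginPlay it caches player pawn 0 as a BP_ThirdPersonCharacter reference.
; Hit events from that character launch it by the platform's own velocity scaled by KnockbackStrength, added to the character's current velocity, then call DamagePlayer with the Damage value.
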(event EventBeginPlay
  ;[0.15 0.15 0.15 0.5] Setup
  (bind _asbp_third_person_character (Utilities|Casting|CastToBP_ThirdPersonCharacter (Game|Player|GetPlayerPawn 0)))
  (Variables|Default|SetPlayerReference _asbp_third_person_character))

(event Collision|EventHit
  (params (MyComp :type Primitive%20Component%20Object%20Reference) (Other :type Actor%20Object%20Reference) (OtherComp :type Primitive%20Component%20Object%20Reference) (bSelfMoved :type Boolean) (HitLocation :type Vector :default "0, 0, 0") (HitNormal :type Vector :default "0, 0, 0") (NormalImpulse :type Vector :default "0, 0, 0") (Hit :type Hit%20Result%20Structure%20%28by%20ref%29))
  ;[1 0.5 0.25 0.5] Knockback Attack
  (if (== Other (Variables|Default|GetPlayerReference))
    (Character|LaunchCharacter (Variables|Default|GetPlayerReference) (* (Transformation|GetVelocity) (Variables|Default|GetKnockbackStrength)) false false)
    ;[1 0.5 0.25 0.5] Damage Player
    (Default|DamagePlayer (Variables|Default|GetPlayerReference) (Variables|Default|GetDamage))))

(fn ConstructionScript)