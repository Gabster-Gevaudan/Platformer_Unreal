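; BP_Skating_Stationary is a platformer obstacle, apparently a stationary variant of a skating hazard, that launches the player on contact.
; On BeginPlay it calls Skate, which plays SkateTimeline with nothing wired to its output.
; Its Hit event launches the player's BP_ThirdPersonCharacter along LaunchDirection, with OverridePlayerVelocity controlling both velocity overrides.
; A leftover, unused Lerp over a spline path length remains in the graph.
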(event Custom|Skate
  (Timeline|Skate%20timeline Play))

(event EventBeginPlay
  (CallFunction|Skate))

(event Collision|EventHit
  (params (MyComp :type Primitive%20Component%20Object%20Reference) (Other :type Actor%20Object%20Reference) (OtherComp :type Primitive%20Component%20Object%20Reference) (bSelfMoved :type Boolean) (HitLocation :type Vector :default "0, 0, 0") (HitNormal :type Vector :default "0, 0, 0") (NormalImpulse :type Vector :default "0, 0, 0") (Hit :type Hit%20Result%20Structure%20%28by%20ref%29))
  (bind _overrideplayervelocity (Variables|Default|GetOverridePlayerVelocity))
  ;[0.4531 1 0.7586 0.5] Jump Pad
  (if (== Other (Game|Player|GetPlayerPawn 0))
    (bind _asbp_third_person_character (Utilities|Casting|CastToBP_ThirdPersonCharacter Other))
    (Character|LaunchCharacter _asbp_third_person_character (Variables|Default|GetLaunchDirection) _overrideplayervelocity _overrideplayervelocity)))

(fn ConstructionScript)